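; BP_P38 is a player-controlled plane that flies forward continuously and fires rockets.
; Tick feeds movement input along the forward vector at a scale that Boost raises while held.
; Pitch and Roll axes rotate the actor locally, and MoveForward adds a local X offset, all scaled by delta time.
; Fire spawns BP_Rocket at the Body's RocketSpawn socket; an unconnected Arrow-based spawn is left over.
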(event EventTick
  (params (DeltaSeconds :type Float%20%28single-precision%29))
  ;[1 1 1] Move Forward
  (Pawn|Input|AddMovementInput (Transformation|GetActorForwardVector) (Variables|Default|GetScale%20Value) false))

(event Input|ActionEvents|InputActionBoost
  (params (Key :type Key%20Structure :default "None"))
  (:Pressed
    (Variables|Default|SetScale%20Value 1.0))
  (:Released
    (Variables|Default|SetScale%20Value 0.5)))

(event Input|ActionEvents|InputActionFire
  (params (Key :type Key%20Structure :default "None"))
  (:Pressed
    (Game|SpawnActorfromClass "/Game/Blueprints/BP_Rocket.BP_Rocket_C" (Transformation|GetSocketTransform (Variables|Default|GetBody) "RocketSpawn" "RTS_World") "Undefined" "MultiplyWithRoot" 0 0)))

(event Input|AxisEvents|InputAxisPitch
  (params (AxisValue :type Float%20%28single-precision%29))
  ;[1 1 1] Pitch
  (Transformation|AddActorLocalRotation (Math|Rotator|MakeRotator 0.0 (* (Math|Float|Clamp(Float) AxisValue -1.0) 6e+01 (Utilities|Time|GetWorldDeltaSeconds)) 0.0) false false))

(event Input|AxisEvents|InputAxisRoll
  (params (AxisValue :type Float%20%28single-precision%29))
  ;[1 1 1] Roll
  (Transformation|AddActorLocalRotation (Math|Rotator|MakeRotator (* (Math|Float|Clamp(Float) AxisValue -1.0) 6e+01 (Utilities|Time|GetWorldDeltaSeconds)) 0.0 0.0) false false))

(event Input|AxisEvents|InputAxisMoveForward
  (params (AxisValue :type Float%20%28single-precision%29))
  ;[1 1 1] Roll
  (Transformation|AddActorLocalOffset (Math|Vector|MakeVector (* (Math|Float|Clamp(Float) AxisValue -1.0) 1.4e+03 (Utilities|Time|GetWorldDeltaSeconds)) 0.0 0.0) false false))

(fn ConstructionScript)